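; BP_LikePlayerController is a player controller Blueprint that turns Enhanced Input actions into pawn movement and look.
; IA_Move adds movement input to player pawn 0 along control-rotation right and forward vectors with pitch zeroed, keeping roll only for the right vector.
; IA_Visual feeds its X and Y values into yaw and pitch input on the controlled pawn.
; BeginPlay and the construction script are empty.
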(event Input|EnhancedActionEvents|EnhancedInputActionIA_Move
  (params (ActionValue :type Vector%202D%20Structure) (ElapsedSeconds :type Float%20%28double-precision%29) (TriggeredSeconds :type Float%20%28double-precision%29) (InputAction :type Input%20Action%20Object%20Reference :default "/Game/Input/IA_Move.IA_Move"))
  (bind _returnvalue (Game|Player|GetPlayerPawn 0))
  (bind _returnvalue_2 (Game|Player|GetPlayerPawn 0))
  (bind _returnvalue_3 (Pawn|GetController _returnvalue_2))
  (bind _returnvalue_4 (Pawn|GetControlRotation _returnvalue_3 :!class /Script/Engine.Controller))
  (:Triggered
    (Pawn|Input|AddMovementInput _returnvalue (Math|Vector|GetRightVector (Math|Rotator|MakeRotator (.roll _returnvalue_4) 0.0 (.yaw _returnvalue_4))) (.x ActionValue) false)
    (Pawn|Input|AddMovementInput _returnvalue (Math|Vector|GetForwardVector (Math|Rotator|MakeRotator 0.0 0.0 (.yaw (Pawn|GetControlRotation (Pawn|GetController _returnvalue_2) :!class /Script/Engine.Controller)))) (.y ActionValue) false)))

(event Input|EnhancedActionEvents|EnhancedInputActionIA_Visual
  (params (ActionValue :type Vector%202D%20Structure) (ElapsedSeconds :type Float%20%28double-precision%29) (TriggeredSeconds :type Float%20%28double-precision%29) (InputAction :type Input%20Action%20Object%20Reference :default "/Game/Input/IA_Visual.IA_Visual"))
  (bind _returnvalue (Pawn|GetControlledPawn))
  (:Triggered
    (Pawn|Input|AddControllerYawInput _returnvalue (.x ActionValue))
    (Pawn|Input|AddControllerPitchInput _returnvalue (.y ActionValue))))

(event EventBeginPlay)

(fn ConstructionScript)